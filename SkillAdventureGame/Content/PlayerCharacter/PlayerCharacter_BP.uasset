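; Player character Blueprint that toggles the inventory screen from the Toggle Inventory input action.
; BeginPlay caches the player controller as PlayerCharacterController_BP for later use.
; Opening creates a new MasterInventory widget each time, adds it to the viewport, sets Game and UI input and shows the cursor.
; Closing removes the widget, restores game-only input and hides the cursor.
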(event `self.ReceiveBeginPlay`
  (bind _asplayer_character_controller_bp (cast `/Game/Controllers/PlayerControllers/PlayerCharacterController_BP` (`GameplayStatics.GetPlayerController` 0)))
  (set `self.ControllerRef` _asplayer_character_controller_bp))

(event `InputAction|Toggle Inventory`
  (params (Key :type "Key Structure"))
  (bind _controllerref (`self.ControllerRef`))
  (bind _controllerref_2 (`self.ControllerRef`))
  (:`Pressed`
    (if (`self.InventoryOpen`)
      (`Widget.RemoveFromParent` (stale _returnvalue))
      (set `self.InventoryOpen` false)
      (`WidgetBlueprintLibrary.SetInputMode_GameOnly` _controllerref_2)
      (set `PlayerController.bShowMouseCursor` false _controllerref_2)
      (else
        (bind _returnvalue (`|CreateWidget` "/Game/HUD_UI/MasterInventory.MasterInventory_C"))
        (`UserWidget.AddToViewport` _returnvalue 0)
        (set `self.InventoryOpen` true)
        (`WidgetBlueprintLibrary.SetInputMode_GameAndUIEx` _controllerref null)
        (set `PlayerController.bShowMouseCursor` true _controllerref)))))

(event `self.ReceiveTick`
  (params (DeltaSeconds :type "Float (single-precision)")))

(fn `UserConstructionScript`)