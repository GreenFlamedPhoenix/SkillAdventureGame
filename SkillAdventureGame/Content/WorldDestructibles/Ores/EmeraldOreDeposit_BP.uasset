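; Destructible emerald ore deposit that drops an emerald chunk pickup or actor when it is destroyed.
; The Destroyed event calls SpawnDepositDrops, which spawns a single EmeraldChunk_BP using the deposit's rotation and scale.
; The chunk lands at a small random positive X/Y offset from the deposit, at a fixed world height rather than one relative to the deposit.
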(event `self.ReceiveDestroyed`
  (`self.SpawnDepositDrops`))

(fn `SpawnDepositDrops`
  (bind _x (.x (.location (`self.GetTransform` self))))
  (bind _y (.y (.location (`self.GetTransform` self))))
  ;[1 1 1] Spawn the chunks
  (`|SpawnActorFromClass` "/Game/Pickups/Ore/EmeraldChunk_BP.EmeraldChunk_BP_C" (`KismetMathLibrary.MakeTransform` (`KismetMathLibrary.MakeVector` (`KismetMathLibrary.RandomFloatInRange` _x (+ _x 10.0)) (`KismetMathLibrary.RandomFloatInRange` _y (+ _y 10.0)) 80.0) (.rotation (`self.GetTransform` self)) (.scale (`self.GetTransform` self))) "Undefined" "OverrideRootScale" null null))

(fn `UserConstructionScript`)