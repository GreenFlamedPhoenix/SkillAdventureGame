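; Destructible iron ore deposit that drops ore chunks when the actor is destroyed.
; The Destroyed event picks a small random count and loops, spawning IronOreChunk_BP actors.
; Each chunk gets a slight random positive X/Y offset from the deposit and inherits its rotation and scale.
; Spawn height is a fixed world Z rather than relative to the deposit.
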(event `self.ReceiveDestroyed`
  (bind _x (.x (.location (`self.GetTransform` self))))
  (bind _y (.y (.location (`self.GetTransform` self))))
  (set `self.DropsToSpawn` (`KismetMathLibrary.RandomIntegerInRange` 1 3))
  (while (> (`self.DropsToSpawn`) 0)
    (`|SpawnActorFromClass` "/Game/Pickups/Ore/IronOreChunk_BP.IronOreChunk_BP_C" (`KismetMathLibrary.MakeTransform` (`KismetMathLibrary.MakeVector` (`KismetMathLibrary.RandomFloatInRange` _x (+ _x 10.0)) (`KismetMathLibrary.RandomFloatInRange` _y (+ _y 10.0)) 75.0) (.rotation (`self.GetTransform` self)) (.scale (`self.GetTransform` self))) "Undefined" "OverrideRootScale" null null)
    (set `self.DropsToSpawn` (- (`self.DropsToSpawn`) 1))))

(fn `UserConstructionScript`)