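; EmeraldChunk_BP is an emerald ore pickup that the player collects by walking into it.
; On BeginPlay it launches its static mesh upward with a random horizontal impulse, scattering it like dropped loot.
; When PlayerCharacter_BP overlaps it, it adds one of its item to that character's InventoryComponent and destroys itself.
; Several disconnected node chains, older inventory-update attempts, remain in the graph but never run.
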(event `self.ReceiveBeginPlay`
  (bind _returnvalue (`KismetMathLibrary.RandomFloatInRange` -250.0 250.0))
  (`PrimitiveComponent.AddImpulse` (`self.StaticMesh`) (`KismetMathLibrary.MakeVector` _returnvalue _returnvalue 500.0) "None" true))

(event `self.ReceiveActorBeginOverlap`
  (params (OtherActor :type "Actor Object Reference"))
  (bind _asplayer_character_bp (cast `/Game/PlayerCharacter/PlayerCharacter_BP` OtherActor))
  (`/Game/PlayerCharacter/TestInventory/InventoryComponent.AddToInventory` (`/Game/PlayerCharacter/PlayerCharacter_BP.InventoryComponent` _asplayer_character_bp) (make `/Game/PlayerCharacter/TestInventory/CraftingInventoryStruct` (`self.ItemPropertiesStructure`) 1))
  (`self.K2_DestroyActor`))

(fn `UserConstructionScript`)